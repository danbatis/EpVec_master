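; Game mode for EpVectors that decides which pawn a player receives by overriding SpawnDefaultPawnFor.
; In the StartGame level it spawns nothing and returns the pawn of player 0.
; In any other level it spawns Player_BP at the first PlayerStart found, ignoring the supplied StartSpot.
; Both branches print debug messages, though the "could not find playerstart" one depends only on level name.
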(event EventBeginPlay)

(event EventTick
  (params (DeltaSeconds :type Float%20%28single-precision%29)))

(fn ConstructionScript)

(fn SpawnDefaultPawnfor
  (params (NewPlayer :type Controller%20Object%20Reference) (StartSpot :type Actor%20Object%20Reference))
  (bind _outactors (Actor|GetAllActorsOfClass "/Script/Engine.PlayerStart"))
  (bind _returnvalue (Game|GetCurrentLevelName true))
  (if (Utilities|Enum|Equal(Enum) _returnvalue "StartGame")
    (Development|PrintString "could not find playerstart")
    (return (Game|Player|GetPlayerPawn 0))
    (else
      (Development|PrintString "found playerStart")
      (bind _returnvalue_2 (Game|SpawnActorfromClass "/Game/EVteam/blueprints/player/Player_BP.Player_BP_C" (Transformation|GetActorTransform (Utilities|Array|Get(acopy) _outactors)) "Undefined" 0 0))
      (return _returnvalue_2))))