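; BasicMutation_BP is a mutation character Blueprint with unfinished logic for being grabbed as a ragdoll and restored afterward.
; BeginPlay caches the mesh's relative rotation and location.
; An unconnected grab chain simulates physics below "joint1" and attaches the mesh at a grabbing socket when the state is Grabbed.
; A second unconnected chain stops simulation, moves the capsule to the mesh, then reattaches it using the cached offsets.
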(event EventBeginPlay
  (bind _mesh (Variables|Character|GetMesh))
  (Variables|Default|SetrotationOffset (Variables|/Script/Engine.SceneComponent|GetRelativeRotation _mesh))
  (Variables|Default|SetpositionOffset (Variables|/Script/Engine.SceneComponent|GetRelativeLocation _mesh)))

(event Collision|EventActorBeginOverlap
  (params (OtherActor :type Actor%20Object%20Reference)))

(event EventTick
  (params (DeltaSeconds :type Float%20%28single-precision%29)))

(fn ConstructionScript)