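; Comic cutscene player actor that pauses the game on BeginPlay, shows a subtitle widget and plays a timed sequence of comic panels.
; Tick accumulates time, spawns a ComicFrame widget for each Frames entry at its spawn time, then drives its fades and linear movement.
; Once playback has started and no panel is live, even if later ones are pending, it unpauses, removes the subtitle and destroys itself.
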(event EventBeginPlay
  (Game|SetGamePaused true)
  (bind _returnvalue (UserInterface|CreateWidget "/Game/EVteam/UI/comicSubtitle.comicSubtitle_C"))
  (Variables|Default|SetsubtitleWidget _returnvalue)
  (UserInterface|Viewport|AddtoViewport _returnvalue 0))

(event Collision|EventActorBeginOverlap
  (params (OtherActor :type Actor%20Object%20Reference)))

(event EventTick
  (params (DeltaSeconds :type Float%20%28single-precision%29))
  (Variables|Default|Setmytime (+ DeltaSeconds (Variables|Default|Getmytime)))
  (if (and (Variables|Default|Getstarted) (not (Variables|Default|GetsomeoneLive)))
    (Game|SetGamePaused false)
    (Widget|RemovefromParent (Variables|Default|GetsubtitleWidget))
    (Actor|DestroyActor)
    (else
      (Variables|Default|SetsomeoneLive false)
      (for (_array_element _array_index) (Variables|Default|Getframes)
        (if (.alive (Utilities|Struct|BreakcomicFrameCfg _array_element))
          ;[1 1 1] travel
          (if (and (>= (Variables|Default|Getmytime) (+ (.spawnTime (Utilities|Struct|BreakcomicFrameCfg _array_element)) (.timeInPos_i (Utilities|Struct|BreakcomicFrameCfg _array_element)))) (<= (Variables|Default|Getmytime) (+ (.spawnTime (Utilities|Struct|BreakcomicFrameCfg _array_element)) (.timeInPos_i (Utilities|Struct|BreakcomicFrameCfg _array_element)) (.time2Travel (Utilities|Struct|BreakcomicFrameCfg _array_element)))))
            (Variables|/Game/EVteam/UI/comicFrame.comicFrame_C|Setposition (.widgetRef (Utilities|Struct|BreakcomicFrameCfg _array_element)) (+ (.pos_i (Utilities|Struct|BreakcomicFrameCfg _array_element)) (* (- (.pos_f (Utilities|Struct|BreakcomicFrameCfg _array_element)) (.pos_i (Utilities|Struct|BreakcomicFrameCfg _array_element))) (/ (- (Variables|Default|Getmytime) (+ (.spawnTime (Utilities|Struct|BreakcomicFrameCfg _array_element)) (.timeInPos_i (Utilities|Struct|BreakcomicFrameCfg _array_element)))) (.time2Travel (Utilities|Struct|BreakcomicFrameCfg _array_element)))))))
          (if (>= (Variables|Default|Getmytime) (+ (.spawnTime (Utilities|Struct|BreakcomicFrameCfg _array_element)) (.fadeInTime (Utilities|Struct|BreakcomicFrameCfg _array_element))))
            (if (>= (Variables|Default|Getmytime) (+ (.spawnTime (Utilities|Struct|BreakcomicFrameCfg _array_element)) (.fadeInTime (Utilities|Struct|BreakcomicFrameCfg _array_element)) (.fullAlphaTime (Utilities|Struct|BreakcomicFrameCfg _array_element)) (.fadeOutTime (Utilities|Struct|BreakcomicFrameCfg _array_element))))
              (Variables|/Game/EVteam/UI/comicFrame.comicFrame_C|Setalpha (.widgetRef (Utilities|Struct|BreakcomicFrameCfg _array_element)) 1.0)
              (Widget|RemovefromParent (.widgetRef (Utilities|Struct|BreakcomicFrameCfg _array_element)))
              (else
                ;[1 1 1] fadeOut
                (Variables|/Game/EVteam/UI/comicFrame.comicFrame_C|Setalpha (.widgetRef (Utilities|Struct|BreakcomicFrameCfg _array_element)) (- 1.0 (/ (- (Variables|Default|Getmytime) (+ (.spawnTime (Utilities|Struct|BreakcomicFrameCfg _array_element)) (.fadeInTime (Utilities|Struct|BreakcomicFrameCfg _array_element)) (.fullAlphaTime (Utilities|Struct|BreakcomicFrameCfg _array_element)))) (.fadeOutTime (Utilities|Struct|BreakcomicFrameCfg _array_element)))))
                (Variables|Default|SetsomeoneLive true)))
            (else
              ;[1 1 1] fadeIn
              (Variables|/Game/EVteam/UI/comicFrame.comicFrame_C|Setalpha (.widgetRef (Utilities|Struct|BreakcomicFrameCfg _array_element)) (/ (- (Variables|Default|Getmytime) (.spawnTime (Utilities|Struct|BreakcomicFrameCfg _array_element))) (.fadeInTime (Utilities|Struct|BreakcomicFrameCfg _array_element))))
              (Variables|Default|SetsomeoneLive true)))
          (else
            ;[1 1 1] SpawnFrame
            (if (>= (Variables|Default|Getmytime) (.spawnTime (Utilities|Struct|BreakcomicFrameCfg _array_element)))
              (bind _returnvalue (UserInterface|CreateWidget "/Game/EVteam/UI/comicFrame.comicFrame_C"))
              (Utilities|Struct|SetmembersincomicFrameCfg (Utilities|Array|Get(acopy) (Variables|Default|Getframes) _array_index) _returnvalue)
              (Variables|/Game/EVteam/UI/comicFrame.comicFrame_C|SetframeTex (.widgetRef (Utilities|Struct|BreakcomicFrameCfg _array_element)) (.frameTex (Utilities|Struct|BreakcomicFrameCfg _array_element)))
              (Variables|/Game/EVteam/UI/comicFrame.comicFrame_C|SetcolorTint (.widgetRef (Utilities|Struct|BreakcomicFrameCfg _array_element)) (.colorTint (Utilities|Struct|BreakcomicFrameCfg _array_element)))
              (Variables|/Game/EVteam/UI/comicFrame.comicFrame_C|Setalpha (.widgetRef (Utilities|Struct|BreakcomicFrameCfg _array_element)) 0.0)
              (Variables|/Game/EVteam/UI/comicFrame.comicFrame_C|Setposition (.widgetRef (Utilities|Struct|BreakcomicFrameCfg _array_element)) (.pos_i (Utilities|Struct|BreakcomicFrameCfg _array_element)))
              (UserInterface|Viewport|AddtoViewport (.widgetRef (Utilities|Struct|BreakcomicFrameCfg _array_element)) 0)
              (Utilities|Struct|SetmembersincomicFrameCfg (Utilities|Array|Get(acopy) (Variables|Default|Getframes) _array_index) true)
              (Variables|Default|Setstarted true)
              (Variables|Default|SetsomeoneLive true))))))))

(fn ConstructionScript)