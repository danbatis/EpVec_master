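; Trigger actor that spawns a group of BasicMutation_BP enemies (mosquitoes) when the player character overlaps it.
; It spawns one mutation at each Places actor and gives it the patrol points from the GoalsS entry at the same index.
; Each spawn is registered with an incrementing index in the game state's mutation list, plus the grappable and grabbable lists when flagged.
; The trigger destroys itself afterwards, so it fires only once.
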(event EventBeginPlay)

(event Collision|EventActorBeginOverlap
  (params (OtherActor :type Actor%20Object%20Reference))
  (Utilities|Casting|CastToMyPlayerCharacter OtherActor)
  (Development|PrintString (Utilities|String|Append "spawning mosquitoes for " (Utilities|GetDisplayName OtherActor)))
  (bind _asvectors_game_state_base (Utilities|Casting|CastToVectorsGameStateBase (Game|GetGameState)))
  (for (_array_element _array_index) (Variables|Default|Getplaces)
    ;[1 1 1] spawn mutation
    (bind _returnvalue (Game|SpawnActorfromClass "/Game/EVteam/blueprints/enemies/BasicMutation_BP.BasicMutation_BP_C" (Transformation|GetActorTransform _array_element) "Undefined" 0 0))
    (Variables|/Script/EpidemicVectors.MutationChar|SetpatrolPoints _returnvalue (Utilities|Struct|BreakpatrolSet (Utilities|Array|Get(acopy) (Variables|Default|Getgoals_s) _array_index)))
    ;[1 1 1] update global enemy list
    (Utilities|Array|Add (Variables|/Script/EpidemicVectors.VectorsGameStateBase|Getmutations _asvectors_game_state_base) _returnvalue)
    (Variables|/Script/EpidemicVectors.MutationChar|Setmutation_i _returnvalue (Variables|/Script/EpidemicVectors.VectorsGameStateBase|Getmutation_i _asvectors_game_state_base))
    (Variables|/Script/EpidemicVectors.VectorsGameStateBase|Setmutation_i _asvectors_game_state_base (+ (Variables|/Script/EpidemicVectors.VectorsGameStateBase|Getmutation_i _asvectors_game_state_base) 1))
    (if (Variables|/Script/EpidemicVectors.MutationChar|Getgrappable _returnvalue)
      (Utilities|Array|Add (Variables|/Script/EpidemicVectors.VectorsGameStateBase|Getgrappables _asvectors_game_state_base) _returnvalue)
      (Variables|/Script/EpidemicVectors.MutationChar|Setgrappable_i _returnvalue (Variables|/Script/EpidemicVectors.VectorsGameStateBase|Getgrappable_i _asvectors_game_state_base))
      (Variables|/Script/EpidemicVectors.VectorsGameStateBase|Setgrappable_i _asvectors_game_state_base (+ (Variables|/Script/EpidemicVectors.VectorsGameStateBase|Getgrappable_i _asvectors_game_state_base) 1)))
    (if (Variables|/Script/EpidemicVectors.MutationChar|Getgrabable _returnvalue)
      (Utilities|Array|Add (Variables|/Script/EpidemicVectors.VectorsGameStateBase|Getgrabables _asvectors_game_state_base) _returnvalue)
      (Variables|/Script/EpidemicVectors.MutationChar|Setgrabable_i _returnvalue (Variables|/Script/EpidemicVectors.VectorsGameStateBase|Getgrabable_i _asvectors_game_state_base))
      (Variables|/Script/EpidemicVectors.VectorsGameStateBase|Setgrabable_i _asvectors_game_state_base (+ (Variables|/Script/EpidemicVectors.VectorsGameStateBase|Getgrabable_i _asvectors_game_state_base) 1))))
  (Actor|DestroyActor))

(event EventTick
  (params (DeltaSeconds :type Float%20%28single-precision%29)))

(fn ConstructionScript)