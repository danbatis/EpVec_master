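; A one-shot trigger prop that sets a new speed on the fleeing mosquito that overlaps it.
; The new speed is PlayerSpeedFactor times the player character's dash speed when Turbo is set, or normal speed otherwise, so it scales with the player's movement.
; It prints a debug message on detecting the mosquito and destroys itself after applying the speed.
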(event EventBeginPlay)

(event Collision|EventActorBeginOverlap
  (params (OtherActor :type Actor%20Object%20Reference))
  (bind _asfleeing_mosquito (Utilities|Casting|CastTofleeingMosquito OtherActor))
  (Development|PrintString (Utilities|String|Append "fleeingMosquito detected: " (Utilities|GetDisplayName _asfleeing_mosquito)) true true "(R=0.000000,G=0.000000,B=0.000000,A=1.000000)")
  (bind _asmy_player_character (Utilities|Casting|CastToMyPlayerCharacter (Game|GetPlayerCharacter 0)))
  (if (Variables|Default|Getturbo)
    (Variables|/Game/EVteam/blueprints/props/fleeingMosquito.fleeingMosquito_C|Setspeed _asfleeing_mosquito (* (Variables|Default|GetplayerSpeedFactor) (Variables|/Script/EpidemicVectors.MyPlayerCharacter|GetdashSpeed _asmy_player_character)))
    (else
      (Variables|/Game/EVteam/blueprints/props/fleeingMosquito.fleeingMosquito_C|Setspeed _asfleeing_mosquito (* (Variables|Default|GetplayerSpeedFactor) (Variables|/Script/EpidemicVectors.MyPlayerCharacter|GetnormalSpeed _asmy_player_character)))))
  (Actor|DestroyActor))

(event EventTick
  (params (DeltaSeconds :type Float%20%28single-precision%29)))

(fn ConstructionScript)