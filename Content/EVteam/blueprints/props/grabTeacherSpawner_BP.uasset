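; Spawner prop, apparently for teaching grabbing by its name, that keeps a BasicMutation enemy in play while Activated.
; Each Tick it sets Active when no mutations exist and no cached water puddle or pool is activated.
; Whenever the GameState mutation list is empty, regardless of the water result, it spawns two air waypoints and a zero-aggressivity mutation patrolling them, then registers it in that list.
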(event EventBeginPlay
  ;[1 1 1] initialize water arrays
  (bind _outactors (Actor|GetAllActorsOfClass "/Game/EVteam/blueprints/enemies/waterpuddle_BP.waterpuddle_BP_C"))
  (Variables|Default|SetwaterPuddles _outactors)
  (bind _outactors_2 (Actor|GetAllActorsOfClass "/Game/EVteam/blueprints/enemies/waterpool_BP.waterpool_BP_C"))
  (Variables|Default|SetwaterPools _outactors_2)
  ;[1 1 1] initialize game state
  (bind _asvectors_game_state_base (Utilities|Casting|CastToVectorsGameStateBase (Game|GetGameState)))
  (Variables|Default|SetgameState _asvectors_game_state_base))

(event Collision|EventActorBeginOverlap
  (params (OtherActor :type Actor%20Object%20Reference)))

(event EventTick
  (params (DeltaSeconds :type Float%20%28single-precision%29))
  (bind _gamestate (Variables|Default|GetgameState))
  (bind _mutations (Variables|/Script/EpidemicVectors.VectorsGameStateBase|Getmutations _gamestate))
  ;[1 1 1] control effect
  (if (Variables|Default|Getactivated)
    (bind _output_get (Variables|Default|Setactive (== (Utilities|Array|Length (Variables|/Script/EpidemicVectors.VectorsGameStateBase|Getmutations (Variables|Default|GetgameState))) 0)))
    (if _output_get
      (bind _array_element (Utilities|Array|ForEachLoopwithBreak (Variables|Default|GetwaterPuddles) :!label _label)
        (:LoopBody
          (Utilities|IsValid _array_element
            (:Is%20Valid
              (if (Variables|/Game/EVteam/blueprints/enemies/waterpuddle_BP.waterpuddle_BP_C|Getactivated _array_element)
                (Variables|Default|Setactive false)
                (goto _label Break)))))
        (:Completed
          (if (Variables|Default|Getactive)
            (bind _array_element_2 (Utilities|Array|ForEachLoopwithBreak (Variables|Default|GetwaterPools) :!label _label_2)
              (:LoopBody
                (Utilities|IsValid _array_element_2
                  (:Is%20Valid
                    (if (Variables|/Game/EVteam/blueprints/enemies/waterpool_BP.waterpool_BP_C|Getactivated _array_element_2)
                      (Variables|Default|Setactive false)
                      (goto _label_2 Break)))))
              (:Completed
                (if (< (Utilities|Array|Length (Variables|/Script/EpidemicVectors.VectorsGameStateBase|Getmutations (Variables|Default|GetgameState))) 1) :!label _label_3
                  ;[1 1 1] create waypoints for new mutation
                  (bind _returnvalue (Game|SpawnActorfromClass "/Script/EpidemicVectors.CustomWaypoint" (Math|Transform|MakeTransform (+ (Transformation|GetActorLocation) (* (Math|Vector|GetUpVector "0, 0, 0") (Variables|Default|GetfirstWaypointHeight)))) "Undefined" 0 0))
                  (Variables|/Script/EpidemicVectors.CustomWaypoint|SetairGoal _returnvalue true)
                  (bind _returnvalue_2 (Game|SpawnActorfromClass "/Script/EpidemicVectors.CustomWaypoint" (Math|Transform|MakeTransform (+ (Transformation|GetActorLocation) (* (Math|Vector|GetUpVector "0, 0, 0") (* 2 (Variables|Default|GetfirstWaypointHeight))) (* (Math|Vector|GetForwardVector "0, 0, 0") (Math|Random|RandomFloatinRange 0.0 (Variables|Default|GetfirstWaypointHeight))) (* (Math|Vector|GetRightVector "0, 0, 0") (Math|Random|RandomFloatinRange 0.0 (Variables|Default|GetfirstWaypointHeight))))) "Undefined" 0 0))
                  (Variables|/Script/EpidemicVectors.CustomWaypoint|SetairGoal _returnvalue_2 true)
                  ;[1 1 1] spawn mutation
                  (bind _returnvalue_3 (Game|SpawnActorfromClass "/Game/EVteam/blueprints/enemies/BasicMutation_BP.BasicMutation_BP_C" (Math|Transform|MakeTransform (Transformation|GetActorLocation)) "Undefined" 0 0))
                  (Variables|/Script/EpidemicVectors.MutationChar|SetpatrolPoints _returnvalue_3 (Utilities|Array|MakeArray _returnvalue _returnvalue_2))
                  ;[1 1 1] update global enemy list
                  (bind _output_get_2 (Variables|Default|SettotalMutations (Utilities|Array|Length _mutations)))
                  (Utilities|Array|Add _mutations _returnvalue_3)
                  (Variables|/Script/EpidemicVectors.MutationChar|Setmutation_i _returnvalue_3 _output_get_2)
                  (Class|MutationChar|StartPatrol _returnvalue_3)
                  (Variables|/Script/EpidemicVectors.MutationChar|Setaggressivity _returnvalue_3 0.0))))
            (else
              (goto _label_3)))))
      (else
        (goto _label_3)))))

(fn ConstructionScript)