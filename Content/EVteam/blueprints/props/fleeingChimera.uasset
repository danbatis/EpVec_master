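; Fleeing chimera AI character for a tailing sequence, moving along an ordered list of goal actors while the player follows.
; Tick advances the goal on proximity, issues a simple move at set speed and bobs the mesh on a sine wave.
; It divides horizontal player distance into bands, writing status and bar distance to the player character.
; Debug drawing and saved-level reload nodes are disconnected, so "restart" only sets status here.
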(event EventBeginPlay
  (Variables|Default|SetplayerCtrl_ue (Game|GetPlayerController 0))
  (bind _asmy_player_character (Utilities|Casting|CastToMyPlayerCharacter (Game|GetPlayerCharacter 0)))
  (bind _output_get (Variables|Default|SetplayerCharCtrl _asmy_player_character))
  (Variables|/Script/EpidemicVectors.MyPlayerCharacter|SetfollwdBarShow _output_get true))

(event Collision|EventActorBeginOverlap
  (params (OtherActor :type Actor%20Object%20Reference)))

(event EventTick
  (params (DeltaSeconds :type Float%20%28single-precision%29))
  (bind _returnvalue (Transformation|GetActorLocation))
  (bind _returnvalue_2 (Transformation|GetActorLocation))
  (bind _playercharctrl (Variables|Default|GetplayerCharCtrl))
  (bind _returnvalue_3 (Transformation|GetActorLocation _playercharctrl))
  (bind _returnvalue_4 (- _returnvalue_3 _returnvalue))
  (bind _returnvalue_5 (Math|Vector|ProjectVectorontoPlane _returnvalue_4 "0, 0,1.000000"))
  (bind _returnvalue_6 (Math|Vector|VectorLength _returnvalue_5))
  (if (and (<= (Math|Vector|VectorLength (- (Transformation|GetActorLocation) (Transformation|GetActorLocation (Utilities|Array|Get(acopy) (Variables|Default|Getgoals) (Variables|Default|Getgoal_i))))) (Variables|Default|GetminDist2Goal)) (< (Variables|Default|Getgoal_i) (- (Utilities|Array|Length (Variables|Default|Getgoals)) 1)))
    (Math|Integer|IncrementInt (Variables|Default|Getgoal_i)
      (:%20%20
        _)))
  (Transformation|SetRelativeLocation (Variables|Character|GetMesh) (* (Math|Vector|GetUpVector "0, 0, 0") (* (Math|Trig|Sin(Radians) (* (Utilities|Time|GetGameTimeinSeconds) (Variables|Default|GetoscilFreq))) (Variables|Default|GetoscilAmp))) false false)
  (Variables|/Script/EpidemicVectors.MyPlayerCharacter|SetfollwdTgtDist (Variables|Default|GetplayerCharCtrl) (/ _returnvalue_6 (* 6 (Variables|/Script/EpidemicVectors.MyPlayerCharacter|GetfollwdTgtStep (Variables|Default|GetplayerCharCtrl)))))
  (Variables|/Script/Engine.CharacterMovementComponent|SetMaxWalkSpeed (Variables|Character|GetCharacterMovement) (Variables|Default|Getspeed))
  (AI|Navigation|SimpleMovetoLocation (AI|GetAIController self) (Transformation|GetActorLocation (Utilities|Array|Get(acopy) (Variables|Default|Getgoals) (Variables|Default|Getgoal_i))))
  (switch int (Math|Float|Truncate (/ _returnvalue_6 (Variables|/Script/EpidemicVectors.MyPlayerCharacter|GetfollwdTgtStep (Variables|Default|GetplayerCharCtrl))))
    (:Default
      (Variables|/Script/EpidemicVectors.MyPlayerCharacter|SetfollwdTgtStatus (Variables|Default|GetplayerCharCtrl) "restart"))
    (:0
      (Variables|/Script/EpidemicVectors.MyPlayerCharacter|SetfollwdTgtStatus (Variables|Default|GetplayerCharCtrl) "wait")
      (Variables|Default|SetdeltaMove (Math|Vector|VectorLength (- _returnvalue_2 (Variables|Default|GetoldPos))) :!label _label)
      (Variables|Default|SetoldPos _returnvalue_2))
    (:1
      (Variables|/Script/EpidemicVectors.MyPlayerCharacter|SetfollwdTgtStatus (Variables|Default|GetplayerCharCtrl) "too close")
      (goto _label))
    (:2
      (Variables|/Script/EpidemicVectors.MyPlayerCharacter|SetfollwdTgtStatus (Variables|Default|GetplayerCharCtrl) "optimal")
      (goto _label))
    (:3
      (Variables|/Script/EpidemicVectors.MyPlayerCharacter|SetfollwdTgtStatus (Variables|Default|GetplayerCharCtrl) "optimal")
      (goto _label))
    (:4
      (Variables|/Script/EpidemicVectors.MyPlayerCharacter|SetfollwdTgtStatus (Variables|Default|GetplayerCharCtrl) "too far")
      (goto _label))
    (:5
      (Variables|/Script/EpidemicVectors.MyPlayerCharacter|SetfollwdTgtStatus (Variables|Default|GetplayerCharCtrl) "get closer")
      (goto _label))))

(fn ConstructionScript)