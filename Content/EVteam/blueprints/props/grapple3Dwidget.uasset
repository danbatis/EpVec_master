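; Grapple prop actor with a 3D widget that keeps turning to face the player character.
; It caches player character 0 on BeginPlay, then each Tick sets the widget's world rotation from a look-at toward that character.
; Only yaw is applied, so the widget stays upright.
; A debug line from widget to player remains in the graph but is disconnected.
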(event EventBeginPlay
  (Variables|Default|SetplayerChar (Game|GetPlayerCharacter 0)))

(event Collision|EventActorBeginOverlap
  (params (OtherActor :type Actor%20Object%20Reference)))

(event EventTick
  (params (DeltaSeconds :type Float%20%28single-precision%29))
  (Transformation|SetWorldRotation (Variables|Default|GetWidget) (Math|Rotator|MakeRotator 0.0 0.0 (.Yaw (Math|Rotator|BreakRotator (Math|Rotator|FindLookatRotation (Transformation|GetWorldLocation (Variables|Default|GetWidget)) (Transformation|GetActorLocation (Variables|Default|GetplayerChar)))))) false false))

(fn ConstructionScript)