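; Checkpoint actor that auto-saves progress and refills life when the player reaches a higher checkpoint ID than the saved one.
; Overlap writes transform, camera rotation, level and tutorial state to "auto-save" and "toLoad" slots, with effects.
; Tick keeps it active only without GameState mutations or activated water puddles and pools, swapping active/inactive FX.
; As a special case, Tick activates a linked grab tutorial after a short delay once unlocked.
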(event EventBeginPlay
  (Variables|Default|SettimeStarted (Utilities|Time|GetTimeSeconds))
  (bind _asmy_player_character (Utilities|Casting|CastToMyPlayerCharacter (Game|GetPlayerCharacter 0)))
  (Variables|Default|SetplayerChar _asmy_player_character)
  ;[1 1 1] initialize water arrays
  (bind _outactors (Actor|GetAllActorsOfClass "/Game/EVteam/blueprints/enemies/waterpuddle_BP.waterpuddle_BP_C"))
  (Variables|Default|SetwaterPuddles _outactors)
  (bind _outactors_2 (Actor|GetAllActorsOfClass "/Game/EVteam/blueprints/enemies/waterpool_BP.waterpool_BP_C"))
  (Variables|Default|SetwaterPools _outactors_2)
  ;[1 1 1] initialize game state
  (bind _asvectors_game_state_base (Utilities|Casting|CastToVectorsGameStateBase (Game|GetGameState)))
  (Variables|Default|SetgameState _asvectors_game_state_base)
  ;[1 1 1] create save game data
  (bind _returnvalue (SaveGame|CreateSaveGameObject "/Game/EVteam/blueprints/props/VectorsSave.VectorsSave_C"))
  (Variables|/Game/EVteam/blueprints/props/VectorsSave.VectorsSave_C|SetcheckPointID _returnvalue (Variables|Default|GetcheckPointID))
  (bind _returnvalue_2 (Game|GetCurrentLevelName true))
  (Variables|/Game/EVteam/blueprints/props/VectorsSave.VectorsSave_C|SetlevelName _returnvalue (Utilities|String|StringToName _returnvalue_2))
  (Variables|Default|SetgameData _returnvalue))

(event Collision|EventActorBeginOverlap
  (params (OtherActor :type Actor%20Object%20Reference))
  (if (Variables|Default|Getactive)
    ;[1 1 1] check if player and if checkpoint ID is bigger than last one
    (bind _returnvalue (SaveGame|LoadGamefromSlot "toLoad"))
    (bind _asvectors_save (Utilities|Casting|CastToVectorsSave _returnvalue))
    (if (> (Variables|Default|GetcheckPointID) (Variables|/Game/EVteam/blueprints/props/VectorsSave.VectorsSave_C|GetcheckPointID _asvectors_save))
      (bind _asmy_player_character (Utilities|Casting|CastToMyPlayerCharacter OtherActor))
      (Variables|Default|SetplayerChar _asmy_player_character)
      ;[1 1 1] write save game data
      (Variables|/Game/EVteam/blueprints/props/VectorsSave.VectorsSave_C|SetcamRotation (Variables|Default|GetgameData) (Transformation|GetActorRotation (Pawn|GetController _asmy_player_character)))
      (Variables|/Game/EVteam/blueprints/props/VectorsSave.VectorsSave_C|SetcheckPointTransform (Variables|Default|GetgameData) (Transformation|GetActorTransform _asmy_player_character))
      (Variables|/Game/EVteam/blueprints/props/VectorsSave.VectorsSave_C|SetinteractionLevel (Variables|Default|GetgameData) (Variables|/Script/EpidemicVectors.MyPlayerCharacter|GetinteractionLevel (Variables|Default|GetplayerChar)))
      (Variables|/Game/EVteam/blueprints/props/VectorsSave.VectorsSave_C|SetgrabTeacherUnlocked (Variables|Default|GetgameData) (Utilities|IsValid (Variables|Default|GetteachGrabBP)))
      ;[1 1 1] write auto-save
      (bind _returnvalue_2 (SaveGame|SaveGametoSlot (Variables|Default|GetgameData) "auto-save"))
      ;[1 1 1] write to-load
      (bind _returnvalue_3 (SaveGame|SaveGametoSlot (Variables|Default|GetgameData) "toLoad"))
      ;[1 1 1] Spawn Save VFX
      (Game|SpawnActorfromClass "/Game/EVteam/VFX/checkpointFXsave.checkpointFXsave_C" (Transformation|GetWorldTransform (Variables|Default|GetFXactive)) "Undefined" 0 0)
      (Audio|PlaySoundatLocation (Variables|Default|GetsaveGameSound) "0, 0, 0" "0, 0, 0" 1.0 1.0 0.0 0 0 0)
      (Variables|/Script/EpidemicVectors.MyPlayerCharacter|Setlife (Variables|Default|GetplayerChar) 1e+02)
      (Variables|Default|SettimeStarted (Utilities|Time|GetTimeSeconds))
      (Utilities|IsValid (Variables|Default|GetteachGrabBP)
        (:Is%20Valid
          (Variables|/Script/EpidemicVectors.VectorsGameStateBase|SetgrabTeacherUnlock (Variables|Default|GetgameState) true))))))

(event EventTick
  (params (DeltaSeconds :type Float%20%28single-precision%29))
  ;[1 1 1] control effect
  (bind _output_get (Variables|Default|Setactive (== (Utilities|Array|Length (Variables|/Script/EpidemicVectors.VectorsGameStateBase|Getmutations (Variables|Default|GetgameState))) 0)))
  (if _output_get
    (bind _array_element (Utilities|Array|ForEachLoopwithBreak (Variables|Default|GetwaterPuddles) :!label _label)
      (:LoopBody
        (Utilities|IsValid _array_element
          (:Is%20Valid
            (if (Variables|/Game/EVteam/blueprints/enemies/waterpuddle_BP.waterpuddle_BP_C|Getactivated _array_element)
              (Variables|Default|Setactive false)
              (goto _label Break)))))
      (:Completed
        (if (Variables|Default|Getactive)
          (bind _array_element_2 (Utilities|Array|ForEachLoopwithBreak (Variables|Default|GetwaterPools) :!label _label_2)
            (:LoopBody
              (Utilities|IsValid _array_element_2
                (:Is%20Valid
                  (if (Variables|/Game/EVteam/blueprints/enemies/waterpool_BP.waterpool_BP_C|Getactivated _array_element_2)
                    (Variables|Default|Setactive false)
                    (goto _label_2 Break)))))
            (:Completed
              (Rendering|SetVisibility (Variables|Default|GetFXactive) (Variables|Default|Getactive) false :!label _label_3)
              (Rendering|SetVisibility (Variables|Default|GetFXinactive) (not (Variables|Default|Getactive)) false)
              ;[1 1 1] Special Case for grab tutorial
              (if (Math|Boolean|ANDBoolean (Variables|Default|Getactive) (Utilities|IsValid (Variables|Default|GetplayerChar)) (>= (Utilities|Time|GetTimeSeconds) (+ (Variables|Default|GettimeStarted) 3.0)) (Variables|/Script/EpidemicVectors.VectorsGameStateBase|GetgrabTeacherUnlock (Variables|Default|GetgameState)))
                (Utilities|IsValid (Variables|Default|GetteachGrabBP)
                  (:Is%20Valid
                    (if (not (Variables|/Game/EVteam/blueprints/props/grabTeacherSpawner_BP.grabTeacherSpawner_BP_C|Getactivated (Variables|Default|GetteachGrabBP)))
                      (Variables|/Script/EpidemicVectors.MyPlayerCharacter|SetinteractionLevel (Variables|Default|GetplayerChar) 5)
                      (Variables|/Game/EVteam/blueprints/props/grabTeacherSpawner_BP.grabTeacherSpawner_BP_C|Setactivated (Variables|Default|GetteachGrabBP) true)))))))
          (else
            (goto _label_3)))))
    (else
      (goto _label_3))))

(fn ConstructionScript)