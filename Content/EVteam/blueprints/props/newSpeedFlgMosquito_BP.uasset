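; Speed flag prop that changes the fleeing mosquito's speed to a multiple of the player's normal speed, or dash speed when Turbo is set.
; A mosquito overlapping it takes that speed unless its PlayerSet flag is already set.
; A player overlapping it applies the speed to the first mosquito found in the level and sets PlayerSet.
; The prop destroys itself once it applies a speed.
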(event EventBeginPlay)

(event Collision|EventActorBeginOverlap
  (params (OtherActor :type Actor%20Object%20Reference))
  (bind _asfleeing_mosquito (Utilities|Casting|CastTofleeingMosquito OtherActor)
    (:then
      (if (not (Variables|/Game/EVteam/blueprints/props/fleeingMosquito.fleeingMosquito_C|GetplayerSet _asfleeing_mosquito))
        (bind _asmy_player_character (Utilities|Casting|CastToMyPlayerCharacter (Game|GetPlayerCharacter 0)))
        (if (Variables|Default|Getturbo)
          (Variables|/Game/EVteam/blueprints/props/fleeingMosquito.fleeingMosquito_C|Setspeed _asfleeing_mosquito (* (Variables|Default|GetplayerSpeedFactor) (Variables|/Script/EpidemicVectors.MyPlayerCharacter|GetdashSpeed _asmy_player_character)))
          (else
            (Variables|/Game/EVteam/blueprints/props/fleeingMosquito.fleeingMosquito_C|Setspeed _asfleeing_mosquito (* (Variables|Default|GetplayerSpeedFactor) (Variables|/Script/EpidemicVectors.MyPlayerCharacter|GetnormalSpeed _asmy_player_character)))))
        (Actor|DestroyActor)))
    (:CastFailed
      (bind _outactors (Actor|GetAllActorsOfClass "/Game/EVteam/blueprints/props/fleeingMosquito.fleeingMosquito_C"))
      (if (> (Utilities|Array|Length _outactors) 0)
        (bind _asmy_player_character_2 (Utilities|Casting|CastToMyPlayerCharacter OtherActor))
        (if (Variables|Default|Getturbo)
          (Variables|/Game/EVteam/blueprints/props/fleeingMosquito.fleeingMosquito_C|Setspeed (Utilities|Array|Get(acopy) _outactors) (* (Variables|Default|GetplayerSpeedFactor) (Variables|/Script/EpidemicVectors.MyPlayerCharacter|GetdashSpeed _asmy_player_character_2)))
          (else
            (Variables|/Game/EVteam/blueprints/props/fleeingMosquito.fleeingMosquito_C|Setspeed (Utilities|Array|Get(acopy) _outactors) (* (Variables|Default|GetplayerSpeedFactor) (Variables|/Script/EpidemicVectors.MyPlayerCharacter|GetnormalSpeed _asmy_player_character_2)))))
        (Variables|/Game/EVteam/blueprints/props/fleeingMosquito.fleeingMosquito_C|SetplayerSet (Utilities|Array|Get(acopy) _outactors) true)
        (Actor|DestroyActor)))))

(event EventTick
  (params (DeltaSeconds :type Float%20%28single-precision%29)))

(fn ConstructionScript)