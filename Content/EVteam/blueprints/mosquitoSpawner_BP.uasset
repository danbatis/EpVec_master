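; Spawner actor that periodically creates BasicMutation_BP enemies at its own transform.
; On BeginPlay a timer is set to SpawnInterval and counts down each Tick.
; When it runs out, the timer resets, a new mutation spawns and receives the spawner's PathPoints as its patrol points.
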(event EventBeginPlay
  (Variables|Default|Settimer (Variables|Default|GetspawnInterval)))

(event Collision|EventActorBeginOverlap
  (params (OtherActor :type Actor%20Object%20Reference)))

(event EventTick
  (params (DeltaSeconds :type Float%20%28single-precision%29))
  (if (<= (Variables|Default|Gettimer) 0.0)
    (Variables|Default|Settimer (Variables|Default|GetspawnInterval))
    (bind _returnvalue (Game|SpawnActorfromClass "/Game/EVteam/blueprints/BasicMutation_BP.BasicMutation_BP_C" (Transformation|GetActorTransform) "Undefined" 0 0))
    (Variables|/Script/EpidemicVectors.MutationChar|SetpatrolPoints _returnvalue (Variables|Default|GetpathPoints))
    (else
      (Variables|Default|Settimer (- (Variables|Default|Gettimer) DeltaSeconds)))))

(fn ConstructionScript)