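; Player character Blueprint that handles sound driven by movement and input.
; Each Tick sets the "loadFactor" float parameter on MyAudio to velocity magnitude divided by DashSpeed, so the audio follows speed.
; Tick also polls player controller 0 directly for a Space Bar press and calls PlaySoundAtLocation.
; A debug print of the speed ratio is left unconnected, and BeginPlay, overlap and construction logic are empty.
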(event EventBeginPlay)

(event Collision|EventActorBeginOverlap
  (params (OtherActor :type Actor%20Object%20Reference)))

(event EventTick
  (params (DeltaSeconds :type Float%20%28single-precision%29))
  (Audio|Parameter|SetFloatParameter (Variables|Default|GetmyAudio) "loadFactor" (/ (Math|Vector|VectorLength (Transformation|GetVelocity)) (Variables|Default|GetdashSpeed)) :!class /Script/Engine.AudioComponent)
  (if (Game|Player|WasInputKeyJustPressed (Game|GetPlayerController 0) "SpaceBar")
    (Audio|PlaySoundatLocation 0 "0, 0, 0" "0, 0, 0" 1.0 1.0 0.0 0 0 0)))

(fn ConstructionScript)