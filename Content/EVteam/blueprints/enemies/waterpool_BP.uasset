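; Water pool enemy spawner that periodically creates basic mutations while activated, until the game state's mutation list reaches a cap.
; Each spawn gets two new airborne waypoints above the pool, the higher randomly offset, then joins the global list and starts patrolling.
; Overlap with a ground punch rip records the pool's ID as dead in every checkpoint, then destroys it with steam effects.
; Debug line and overlap print remain active.
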(event EventBeginPlay
  (Variables|Default|SetspawnTimer (Variables|Default|GetspawnRate))
  (bind _asvectors_game_state_base (Utilities|Casting|CastToVectorsGameStateBase (Game|GetGameState)))
  (Variables|Default|SetgameState _asvectors_game_state_base)
  (bind _outactors (Actor|GetAllActorsOfClass "/Game/EVteam/blueprints/props/checkPoint_BP.checkPoint_BP_C"))
  (Variables|Default|Setcheckpoints _outactors))

(event Collision|EventActorBeginOverlap
  (params (OtherActor :type Actor%20Object%20Reference))
  (bind _poolmesh (Variables|Default|GetpoolMesh))
  (bind _returnvalue (Transformation|GetWorldLocation _poolmesh))
  (Development|PrintString (Utilities|String|Append "overlapping: " (Utilities|GetDisplayName OtherActor)) true true "(R=1.000000,G=0.008333,B=0.030809,A=1.000000)")
  (Utilities|Casting|CastTogroundPunchRip_BP OtherActor)
  (for _array_element (Variables|Default|Getcheckpoints)
    (Utilities|Array|Add (Variables|/Game/EVteam/blueprints/props/VectorsSave.VectorsSave_C|GetdeadPools (Variables|/Game/EVteam/blueprints/props/checkPoint_BP.checkPoint_BP_C|GetgameData _array_element)) (Variables|Default|GetID)))
  (Effects|SpawnEmitteratLocation "/Game/EVteam/VFX/ParticleSystems/puddleSteam.puddleSteam" _returnvalue)
  (Audio|PlaySoundatLocation "/Game/EVteam/audio/SFX/puddleSteam.puddleSteam" _returnvalue "0, 0, 0" 1.0 1.0 0.0 0 0 0)
  (Actor|DestroyActor))

(event EventTick
  (params (DeltaSeconds :type Float%20%28single-precision%29))
  (bind _returnvalue (Transformation|GetActorLocation))
  (bind _gamestate (Variables|Default|GetgameState))
  (bind _mutations (Variables|/Script/EpidemicVectors.VectorsGameStateBase|Getmutations _gamestate))
  (if (Variables|Default|Getactivated)
    (Rendering|Debug|DrawDebugLine _returnvalue (+ _returnvalue (* (Math|Vector|GetUpVector "0, 0, 0") 1e+03)) "(R=0.000000,G=1.000000,B=0.086108,A=1.000000)" 0.0 0.0)
    (if (<= (Variables|Default|GetspawnTimer) 0.0)
      (if (<= (Utilities|Array|Length (Variables|/Script/EpidemicVectors.VectorsGameStateBase|Getmutations (Variables|Default|GetgameState))) (- (Variables|Default|GetmaxMutations2Spawn) 1))
        (Variables|Default|SetspawnTimer (Variables|Default|GetspawnRate))
        ;[1 1 1] create waypoints for new mutation
        (bind _returnvalue_2 (Game|SpawnActorfromClass "/Script/EpidemicVectors.CustomWaypoint" (Math|Transform|MakeTransform (+ (Transformation|GetActorLocation) (* (Math|Vector|GetUpVector "0, 0, 0") (Variables|Default|GetfirstWaypointHeight)))) "Undefined" 0 0))
        (Variables|/Script/EpidemicVectors.CustomWaypoint|SetairGoal _returnvalue_2 true)
        (bind _returnvalue_3 (Game|SpawnActorfromClass "/Script/EpidemicVectors.CustomWaypoint" (Math|Transform|MakeTransform (+ (Transformation|GetActorLocation) (* (Math|Vector|GetUpVector "0, 0, 0") (* 2 (Variables|Default|GetfirstWaypointHeight))) (* (Math|Vector|GetForwardVector "0, 0, 0") (Math|Random|RandomFloatinRange 0.0 (Variables|Default|GetfirstWaypointHeight))) (* (Math|Vector|GetRightVector "0, 0, 0") (Math|Random|RandomFloatinRange 0.0 (Variables|Default|GetfirstWaypointHeight))))) "Undefined" 0 0))
        (Variables|/Script/EpidemicVectors.CustomWaypoint|SetairGoal _returnvalue_3 true)
        ;[1 1 1] spawn mutation
        (bind _returnvalue_4 (Game|SpawnActorfromClass "/Game/EVteam/blueprints/enemies/BasicMutation_BP.BasicMutation_BP_C" (Math|Transform|MakeTransform (+ (Transformation|GetActorLocation) "0, 0,100.000000")) "Undefined" 0 0))
        (Variables|/Script/EpidemicVectors.MutationChar|SetpatrolPoints _returnvalue_4 (Utilities|Array|MakeArray _returnvalue_2 _returnvalue_3))
        ;[1 1 1] update global enemy list
        (bind _output_get (Variables|Default|SettotalMutations (Utilities|Array|Length _mutations)))
        (Utilities|Array|Add _mutations _returnvalue_4)
        (Variables|/Script/EpidemicVectors.MutationChar|Setmutation_i _returnvalue_4 _output_get)
        (Class|MutationChar|StartPatrol _returnvalue_4))
      (else
        (Variables|Default|SetspawnTimer (- (Variables|Default|GetspawnTimer) DeltaSeconds))))))

(fn ConstructionScript)