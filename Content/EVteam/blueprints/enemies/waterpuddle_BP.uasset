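; Water puddle actor that evaporates when a groundPunchRip_BP overlaps it, playing a steam effect and sound before destroying itself.
; It caches every CheckPoint_BP on BeginPlay and, on death, adds its ID to each checkpoint's GameData DeadPuddles list.
; While Activated, Tick draws a blue debug line straight up from the puddle.
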(event EventBeginPlay
  (bind _outactors (Actor|GetAllActorsOfClass "/Game/EVteam/blueprints/props/checkPoint_BP.checkPoint_BP_C"))
  (Variables|Default|Setcheckpoints _outactors))

(event Collision|EventActorBeginOverlap
  (params (OtherActor :type Actor%20Object%20Reference))
  (bind _waterpuddle (Variables|Default|GetwaterPuddle))
  (bind _returnvalue (Transformation|GetWorldLocation _waterpuddle))
  (Utilities|Casting|CastTogroundPunchRip_BP OtherActor)
  (for _array_element (Variables|Default|Getcheckpoints)
    (Utilities|Array|Add (Variables|/Game/EVteam/blueprints/props/VectorsSave.VectorsSave_C|GetdeadPuddles (Variables|/Game/EVteam/blueprints/props/checkPoint_BP.checkPoint_BP_C|GetgameData _array_element)) (Variables|Default|GetID)))
  (Effects|SpawnEmitteratLocation "/Game/EVteam/VFX/ParticleSystems/puddleSteam.puddleSteam" _returnvalue)
  (Audio|PlaySoundatLocation "/Game/EVteam/audio/SFX/puddleSteam.puddleSteam" _returnvalue "0, 0, 0" 1.0 1.0 0.0 0 0 0)
  (Actor|DestroyActor))

(event EventTick
  (params (DeltaSeconds :type Float%20%28single-precision%29))
  (bind _returnvalue (Transformation|GetActorLocation))
  (if (Variables|Default|Getactivated)
    (Rendering|Debug|DrawDebugLine _returnvalue (+ _returnvalue (* (Math|Vector|GetUpVector "0, 0, 0") 1e+03)) "(R=0.018909,G=0.352940,B=1.000000,A=1.000000)" 0.0 0.0)))

(fn ConstructionScript)