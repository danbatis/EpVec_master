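; Trigger actor that switches on linked water pool, puddle, egg and egg shell actors when the player enters it.
; On overlap with MyPlayerCharacter, it sets the Activated flag on the single Waterpool and on every valid entry in the Waterpuddles, Eggs and EggShells arrays.
; It then destroys itself, making it a one-shot trigger.
; A debug string names every overlapping actor, player or not.
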(event EventBeginPlay)

(event Collision|EventActorBeginOverlap
  (params (OtherActor :type Actor%20Object%20Reference))
  (Development|PrintString (Utilities|String|Append "just entered: " (Utilities|GetDisplayName OtherActor)))
  ;[1 1 1] activates water puddles, eggs and self destruct
  (Utilities|Casting|CastToMyPlayerCharacter OtherActor)
  (Utilities|IsValid (Variables|Default|Getwaterpool)
    (:Is%20Valid
      (Variables|/Game/EVteam/blueprints/enemies/waterpool_BP.waterpool_BP_C|Setactivated (Variables|Default|Getwaterpool) true))
    (:Is%20Not%20Valid
      _))
  (for _array_element (Variables|Default|Getwaterpuddles)
    (Utilities|IsValid _array_element
      (:Is%20Valid
        (Variables|/Game/EVteam/blueprints/enemies/waterpuddle_BP.waterpuddle_BP_C|Setactivated _array_element true))))
  (for _array_element_2 (Variables|Default|Geteggs)
    (Utilities|IsValid _array_element_2
      (:Is%20Valid
        (Variables|/Game/EVteam/blueprints/enemies/MosquitoEgg_BP.MosquitoEgg_BP_C|Setactivated _array_element_2 true))))
  (for _array_element_3 (Variables|Default|GeteggShells)
    (Utilities|IsValid _array_element_3
      (:Is%20Valid
        (Variables|/Game/EVteam/blueprints/enemies/MosquitoEggShell_BP.MosquitoEggShell_BP_C|Setactivated _array_element_3 true))))
  (Actor|DestroyActor))

(event EventTick
  (params (DeltaSeconds :type Float%20%28single-precision%29)))

(fn ConstructionScript)