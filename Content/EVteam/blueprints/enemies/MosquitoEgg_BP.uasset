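; Mosquito egg enemy that loses life when the player or a ground-punch rip overlaps it, with hit FX, and is destroyed at zero.
; A surviving player hit spawns a BasicMutation at the egg with two air waypoints above it as patrol points, the second randomly offset.
; The mutation registers in the VectorsGameStateBase Mutations list and stores its index.
; Ground-punch hits deal heavier damage and spawn nothing beyond the FX.
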(event EventBeginPlay)

(event Collision|EventActorBeginOverlap
  (params (OtherActor :type Actor%20Object%20Reference))
  (Development|PrintString (Utilities|String|Append "egg overlap: " (Utilities|GetDisplayName OtherActor)) true true "(R=1.000000,G=0.586843,B=0.055275,A=1.000000)")
  (Utilities|Casting|CastToMyPlayerCharacter OtherActor
    (:then
      (bind _output_get (Variables|Default|SeteggLife (- (Variables|Default|GeteggLife) 2e+01)))
      (Effects|SpawnEmitteratLocation "/Game/EVteam/VFX/ParticleSystems/eggHitFX.eggHitFX" (Transformation|GetActorLocation))
      (if (<= _output_get 0.0)
        (Actor|DestroyActor)
        (else
          ;[1 1 1] create waypoints for new mutation
          (bind _asvectors_game_state_base (Utilities|Casting|CastToVectorsGameStateBase (Game|GetGameState)))
          (bind _returnvalue (Game|SpawnActorfromClass "/Script/EpidemicVectors.CustomWaypoint" (Math|Transform|MakeTransform (+ (Transformation|GetActorLocation) (* (Math|Vector|GetUpVector "0, 0, 0") (Variables|Default|GetfirstWaypointHeight)))) "Undefined" 0 0))
          (Variables|/Script/EpidemicVectors.CustomWaypoint|SetairGoal _returnvalue true)
          (bind _returnvalue_2 (Game|SpawnActorfromClass "/Script/EpidemicVectors.CustomWaypoint" (Math|Transform|MakeTransform (+ (Transformation|GetActorLocation) (* (Math|Vector|GetUpVector "0, 0, 0") (* 2 (Variables|Default|GetfirstWaypointHeight))) (* (Math|Vector|GetForwardVector "0, 0, 0") (Math|Random|RandomFloatinRange 0.0 (Variables|Default|GetfirstWaypointHeight))) (* (Math|Vector|GetRightVector "0, 0, 0") (Math|Random|RandomFloatinRange 0.0 (Variables|Default|GetfirstWaypointHeight))))) "Undefined" 0 0))
          (Variables|/Script/EpidemicVectors.CustomWaypoint|SetairGoal _returnvalue_2 true)
          ;[1 1 1] spawn mutation
          (bind _returnvalue_3 (Game|SpawnActorfromClass "/Game/EVteam/blueprints/enemies/BasicMutation_BP.BasicMutation_BP_C" (Math|Transform|MakeTransform (Transformation|GetActorLocation)) "Undefined" 0 0))
          (Variables|/Script/EpidemicVectors.MutationChar|SetpatrolPoints _returnvalue_3 (Utilities|Array|MakeArray _returnvalue _returnvalue_2))
          ;[1 1 1] update global enemy list
          (Utilities|Array|Add (Variables|/Script/EpidemicVectors.VectorsGameStateBase|Getmutations _asvectors_game_state_base) _returnvalue_3)
          (Variables|/Script/EpidemicVectors.MutationChar|Setmutation_i _returnvalue_3 (- (Utilities|Array|Length (Variables|/Script/EpidemicVectors.VectorsGameStateBase|Getmutations _asvectors_game_state_base)) 1)))))
    (:CastFailed
      (Utilities|Casting|CastTogroundPunchRip_BP OtherActor)
      (bind _output_get_2 (Variables|Default|SeteggLife (- (Variables|Default|GeteggLife) 4e+01)))
      (Effects|SpawnEmitteratLocation "/Game/EVteam/VFX/ParticleSystems/eggHitFX.eggHitFX" (Transformation|GetActorLocation))
      (if (<= _output_get_2 0.0)
        (Actor|DestroyActor)))))

(event EventTick
  (params (DeltaSeconds :type Float%20%28single-precision%29)))

(fn ConstructionScript)