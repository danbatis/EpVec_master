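; SpawnMosquitos_BP is a one-shot trigger that spawns mosquito enemies when the player character overlaps it.
; It spawns a BasicMutation_BP at each Places actor's transform and assigns patrol points from the GoalsS entry at the same index.
; Each mutation joins the VectorsGameStateBase Mutations list, stores its index there and starts patrolling.
; The trigger destroys itself after the spawn loop.
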(event EventBeginPlay)

(event Collision|EventActorBeginOverlap
  (params (OtherActor :type Actor%20Object%20Reference))
  (Utilities|Casting|CastToMyPlayerCharacter OtherActor)
  (Development|PrintString (Utilities|String|Append "spawning mosquitoes for " (Utilities|GetDisplayName OtherActor)))
  (bind _asvectors_game_state_base (Utilities|Casting|CastToVectorsGameStateBase (Game|GetGameState)))
  (for (_array_element _array_index) (Variables|Default|Getplaces)
    ;[1 1 1] spawn mutation
    (bind _returnvalue (Game|SpawnActorfromClass "/Game/EVteam/blueprints/enemies/BasicMutation_BP.BasicMutation_BP_C" (Transformation|GetActorTransform _array_element) "Undefined" 0 0))
    (Variables|/Script/EpidemicVectors.MutationChar|SetpatrolPoints _returnvalue (Utilities|Struct|BreakpatrolSet (Utilities|Array|Get(acopy) (Variables|Default|Getgoals_s) _array_index)))
    ;[1 1 1] update global enemy list
    (Utilities|Array|Add (Variables|/Script/EpidemicVectors.VectorsGameStateBase|Getmutations _asvectors_game_state_base) _returnvalue)
    (Variables|/Script/EpidemicVectors.MutationChar|Setmutation_i _returnvalue (- (Utilities|Array|Length (Variables|/Script/EpidemicVectors.VectorsGameStateBase|Getmutations _asvectors_game_state_base)) 1))
    (Class|MutationChar|StartPatrol _returnvalue))
  (Actor|DestroyActor))

(event EventTick
  (params (DeltaSeconds :type Float%20%28single-precision%29)))

(fn ConstructionScript)