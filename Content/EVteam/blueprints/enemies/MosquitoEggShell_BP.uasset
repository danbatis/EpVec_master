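; MosquitoEggShell_BP is a destructible mosquito egg shell that loses life when overlapped by the player or, more heavily, by a ground punch rip.
; Each hit spawns a hit effect; at zero life it adds its ID to the dead egg shell list in every cached checkpoint's game data, then destroys itself.
; While activated, it draws a vertical debug line from its location every tick.
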(event EventBeginPlay
  (bind _outactors (Actor|GetAllActorsOfClass "/Game/EVteam/blueprints/props/checkPoint_BP.checkPoint_BP_C"))
  (Variables|Default|Setcheckpoints _outactors))

(event Collision|EventActorBeginOverlap
  (params (OtherActor :type Actor%20Object%20Reference))
  (Utilities|Casting|CastToMyPlayerCharacter OtherActor
    (:then
      (bind _output_get (Variables|Default|SeteggLife (- (Variables|Default|GeteggLife) 2e+01)))
      (Effects|SpawnEmitteratLocation "/Game/EVteam/VFX/ParticleSystems/eggHitFX.eggHitFX" (Transformation|GetActorLocation))
      (if (<= _output_get 0.0)
        (for _array_element (Variables|Default|Getcheckpoints) :!label _label
          (Utilities|Array|Add (Variables|/Game/EVteam/blueprints/props/VectorsSave.VectorsSave_C|GetdeadEggShells (Variables|/Game/EVteam/blueprints/props/checkPoint_BP.checkPoint_BP_C|GetgameData _array_element)) (Variables|Default|GetID)))
        (Actor|DestroyActor)))
    (:CastFailed
      (Utilities|Casting|CastTogroundPunchRip_BP OtherActor)
      (bind _output_get_2 (Variables|Default|SeteggLife (- (Variables|Default|GeteggLife) 4e+01)))
      (Effects|SpawnEmitteratLocation "/Game/EVteam/VFX/ParticleSystems/eggHitFX.eggHitFX" (Transformation|GetActorLocation))
      (if (<= _output_get_2 0.0)
        (goto _label)))))

(event EventTick
  (params (DeltaSeconds :type Float%20%28single-precision%29))
  (bind _returnvalue (Transformation|GetActorLocation))
  (if (Variables|Default|Getactivated)
    (Rendering|Debug|DrawDebugLine _returnvalue (+ _returnvalue (* (Math|Vector|GetUpVector "0, 0, 0") 1e+03)) "(R=0.109625,G=1.000000,B=0.000000,A=1.000000)" 0.0 0.0)))

(fn ConstructionScript)