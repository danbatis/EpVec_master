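; AdjustInteractionLevel_BP is a one-shot trigger actor that sets the player character's InteractionLevel to its NewIntLevel value.
; BeginPlay caches player 0's MyPlayerCharacter, with a cast of the overlapping actor as fallback when that reference is invalid.
; On overlap it writes the level and destroys itself; with a valid cached player, any overlapping actor triggers this.
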(event EventBeginPlay
  (bind _asmy_player_character (Utilities|Casting|CastToMyPlayerCharacter (Game|GetPlayerCharacter 0)))
  (Variables|Default|SetplayerCtrl _asmy_player_character))

(event Collision|EventActorBeginOverlap
  (params (OtherActor :type Actor%20Object%20Reference))
  (if (Utilities|IsValid (Variables|Default|GetplayerCtrl))
    _
    (else
      (bind _asmy_player_character (Utilities|Casting|CastToMyPlayerCharacter OtherActor))
      (bind _output_get (Variables|Default|SetplayerCtrl _asmy_player_character))))
  (Variables|/Script/EpidemicVectors.MyPlayerCharacter|SetinteractionLevel (Variables|Default|GetplayerCtrl) (Variables|Default|GetnewIntLevel))
  (Actor|DestroyActor))

(event EventTick
  (params (DeltaSeconds :type Float%20%28single-precision%29)))

(fn ConstructionScript)