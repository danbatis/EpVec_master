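; Ground punch ripple actor for the player that damages and likely knocks down BasicMutation_BP enemies it overlaps.
; Tick moves RippleMesh in a hand-computed arc, using constant forward speed and a vertical speed that starts at Vzero and decreases by DownRate.
; It destroys itself once the next position would fall more than 100 units below its spawn height.
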(event EventBeginPlay
  (Variables|Default|SetupSpeed (Variables|Default|Getvzero))
  (Variables|Default|SetmyTransform (Transformation|GetWorldTransform (Variables|Default|GetRippleMesh)))
  (Variables|Default|SetinitialPos (Transformation|GetActorLocation)))

(event Collision|EventActorBeginOverlap
  (params (OtherActor :type Actor%20Object%20Reference))
  (bind _asbasic_mutation_bp (Utilities|Casting|CastToBasicMutation_BP OtherActor))
  (Class|MutationChar|MyDamage _asbasic_mutation_bp 5.0 (Transformation|GetActorLocation) true 1.0 0.0 (Transformation|GetActorLocation _asbasic_mutation_bp) "0, 0,1.000000"))

(event EventTick
  (params (DeltaSeconds :type Float%20%28single-precision%29))
  (bind _output_get (Variables|Default|SetupSpeed (- (Variables|Default|GetupSpeed) (* (Variables|Default|GetdownRate) DeltaSeconds))))
  (if (>= (.Z (Math|Vector|BreakVector (+ (.Location (Math|Transform|BreakTransform (Variables|Default|GetmyTransform))) (* (Math|Vector|GetUpVector "0, 0, 0") (* _output_get DeltaSeconds)) (* (Transformation|GetActorForwardVector) (* (Variables|Default|GetforthSpeed) DeltaSeconds))))) (- (.Z (Math|Vector|BreakVector (Variables|Default|GetinitialPos))) 1e+02))
    (bind _output_get_2 (Variables|Default|SetmyTransform (Math|Transform|MakeTransform (+ (.Location (Math|Transform|BreakTransform (Variables|Default|GetmyTransform))) (* (Math|Vector|GetUpVector "0, 0, 0") (* _output_get DeltaSeconds)) (* (Transformation|GetActorForwardVector) (* (Variables|Default|GetforthSpeed) DeltaSeconds))) (.Rotation (Math|Transform|BreakTransform (Variables|Default|GetmyTransform))) (.Scale (Math|Transform|BreakTransform (Variables|Default|GetmyTransform))))))
    (Transformation|SetWorldTransform (Variables|Default|GetRippleMesh) _output_get_2 false false)
    (else
      (Actor|DestroyActor))))

(fn ConstructionScript)