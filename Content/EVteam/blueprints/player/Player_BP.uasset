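; Player character Blueprint that handles startup, checkpoint restore, skill tutorials and debug keys.
; BeginPlay caches VFX and ambient sound references, adds the UI, then loads the save to restore transform, camera and progress, destroying previously cleared mosquito and water actors.
; Tick feeds speed to thrust audio, matches global pitch to time dilation and spawns tutorial actors as SkillLevel and readiness flags change.
; Keys pause, reload or reset the level, adjust InteractionLevel and test comics and pitch.
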(event EventBeginPlay
  (bind _outactors (Actor|GetAllActorsOfClass "/Script/Engine.AmbientSound"))
  (Variables|Default|SetambSoundRef (Utilities|Array|Get(acopy) _outactors))
  ;[1 1 1] initialize game state
  (bind _asvectors_game_state_base (Utilities|Casting|CastToVectorsGameStateBase (Game|GetGameState)))
  (Variables|Default|SetgameState _asvectors_game_state_base)
  ;[1 1 1] VFX inits
  (Variables|Default|SetjetBackUp (Variables|Default|GetjetMainUpper))
  (Variables|Default|SetjetBackLow (Variables|Default|GetjetMainLower))
  (Variables|Default|SetjetBackL (Variables|Default|GetbackJetFXL))
  (Variables|Default|SetjetLegL (Variables|Default|GetlegJetFXL))
  (Variables|Default|SetjetBackR (Variables|Default|GetbackJetFXR))
  (Variables|Default|SetjetLegR (Variables|Default|GetlegJetFXR))
  (Variables|Default|SetturboThrustVFX (Variables|Default|GetturboThrustFX))
  (Variables|Default|SetmainThrustVFX (Variables|Default|GetmainThrustFX))
  (Variables|Default|SetswordVFX (Variables|Default|GetswordTrail))
  (Variables|Default|SetclawVFX (Variables|Default|GethookTrail))
  (Variables|Default|SetrangedSwordVFX (Variables|Default|GetrangedSwordTrail))
  (Variables|Default|SetgroundPunchVFX (Variables|Default|GetgroundPunchTrail))
  (bind _output_get (Variables|Default|SethookChain (Variables|Default|Getchain)))
  (Components|Activation|Deactivate _output_get)
  ;[1 1 1] ADD UI
  (bind _returnvalue (UserInterface|CreateWidget "/Game/EVteam/UI/BasicUI.BasicUI_C" (Game|GetPlayerController 0)))
  (UserInterface|Viewport|AddtoViewport _returnvalue 0)
  (Variables|Default|SetplayerUI _returnvalue)
  (bind _returnvalue_2 (Game|GetCurrentLevelName true))
  (if (Utilities|Enum|Equal(Enum) _returnvalue_2 "InitialPursuit")
    (Development|PrintString "first level!")
    (else
      (Development|PrintString "disable grab teach")
      (Variables|Default|SetgrabThrowLearned true)))
  ;[1 1 1] SaveSystem teleport to checkpoint
  (bind _returnvalue_3 (SaveGame|DoesSaveGameExist "toLoad"))
  (if (and _returnvalue_3 (Variables|Default|GetsaveSystem))
    (bind _returnvalue_4 (SaveGame|LoadGamefromSlot "toLoad"))
    (bind _asvectors_save (Utilities|Casting|CastToVectorsSave _returnvalue_4))
    (bind _returnvalue_5 (Game|GetCurrentLevelName true))
    (if (and (Utilities|Enum|Equal(Enum) _returnvalue_5 (Variables|/Game/EVteam/blueprints/props/VectorsSave.VectorsSave_C|GetlevelName _asvectors_save)) (> (Variables|/Game/EVteam/blueprints/props/VectorsSave.VectorsSave_C|GetcheckPointID _asvectors_save) 0))
      (Transformation|SetActorTransform (Variables|/Game/EVteam/blueprints/props/VectorsSave.VectorsSave_C|GetcheckPointTransform _asvectors_save))
      (Pawn|SetControlRotation (Pawn|GetController) (Variables|/Game/EVteam/blueprints/props/VectorsSave.VectorsSave_C|GetcamRotation _asvectors_save))
      (bind _output_get_2 (Variables|/Script/EpidemicVectors.VectorsGameStateBase|SetcheckpointID (Variables|Default|GetgameState) (Variables|/Game/EVteam/blueprints/props/VectorsSave.VectorsSave_C|GetinteractionLevel _asvectors_save)))
      (Variables|Default|SetinteractionLevel _output_get_2)
      (Variables|Default|SetskillLevel (Variables|/Game/EVteam/blueprints/props/VectorsSave.VectorsSave_C|GetskillLevel _asvectors_save))
      (Variables|Default|SetlessonsLearned (Variables|/Game/EVteam/blueprints/props/VectorsSave.VectorsSave_C|GetlessonsLearned _asvectors_save))
      (Variables|/Script/EpidemicVectors.VectorsGameStateBase|SetgrabTeacherUnlock (Variables|Default|GetgameState) (Variables|/Game/EVteam/blueprints/props/VectorsSave.VectorsSave_C|GetgrabTeacherUnlocked _asvectors_save))
      (if (Variables|/Game/EVteam/blueprints/props/VectorsSave.VectorsSave_C|GetgrabTeacherUnlocked _asvectors_save)
        (Variables|Default|SetinteractionLevel 5)
        ;[1 1 1] Deleting already destroyed elements
        (bind _outactors_2 (Actor|GetAllActorsOfClass "/Game/EVteam/blueprints/enemies/MosquitoEggShell_BP.MosquitoEggShell_BP_C"))
        (for _array_element _outactors_2
          (if (Utilities|Array|ContainsItem (Variables|/Game/EVteam/blueprints/props/VectorsSave.VectorsSave_C|GetdeadEggShells _asvectors_save) (Variables|/Game/EVteam/blueprints/enemies/MosquitoEggShell_BP.MosquitoEggShell_BP_C|GetID _array_element))
            (Actor|DestroyActor _array_element)))
        (bind _outactors_3 (Actor|GetAllActorsOfClass "/Game/EVteam/blueprints/enemies/MosquitoEgg_BP.MosquitoEgg_BP_C"))
        (for _array_element_2 _outactors_3
          (if (Utilities|Array|ContainsItem (Variables|/Game/EVteam/blueprints/props/VectorsSave.VectorsSave_C|GetdeadEggs _asvectors_save) (Variables|/Game/EVteam/blueprints/enemies/MosquitoEgg_BP.MosquitoEgg_BP_C|GetID _array_element_2))
            (Actor|DestroyActor _array_element_2)))
        (bind _outactors_4 (Actor|GetAllActorsOfClass "/Game/EVteam/blueprints/enemies/waterpool_BP.waterpool_BP_C"))
        (for _array_element_3 _outactors_4
          (if (Utilities|Array|ContainsItem (Variables|/Game/EVteam/blueprints/props/VectorsSave.VectorsSave_C|GetdeadPools _asvectors_save) (Variables|/Game/EVteam/blueprints/enemies/waterpool_BP.waterpool_BP_C|GetID _array_element_3))
            (Actor|DestroyActor _array_element_3)))
        (bind _outactors_5 (Actor|GetAllActorsOfClass "/Game/EVteam/blueprints/enemies/waterpuddle_BP.waterpuddle_BP_C"))
        (for _array_element_4 _outactors_5
          (if (Utilities|Array|ContainsItem (Variables|/Game/EVteam/blueprints/props/VectorsSave.VectorsSave_C|GetdeadPuddles _asvectors_save) (Variables|/Game/EVteam/blueprints/enemies/waterpuddle_BP.waterpuddle_BP_C|GetID _array_element_4))
            (Actor|DestroyActor _array_element_4)))))))

(event Collision|EventActorBeginOverlap
  (params (OtherActor :type Actor%20Object%20Reference)))

(event EventTick
  (params (DeltaSeconds :type Float%20%28single-precision%29))
  ;[1 1 1] Setting speed for variable thrust sound and some tutorial management
  (Audio|Parameter|SetFloatParameter (Variables|Default|GetmyAudio) "loadFactor" (/ (Math|Vector|VectorLength (Transformation|GetVelocity)) (Variables|Default|GetdashSpeed)) :!class /Script/Engine.AudioComponent)
  (if (== (Variables|Default|GettimeDilation) 1.0)
    (Class|GameplayStatics|SetGlobalPitchModulation (Variables|Default|GettimeDilation) 0.0)
    (else
      (Class|GameplayStatics|SetGlobalPitchModulation (* (Variables|Default|GettimeDilation) 4.0) 0.0)))
  (if (Variables|Default|Getready4newSkill)
    (switch int (Variables|Default|GetskillLevel)
      (:0
        (bind _returnvalue (Game|SpawnActorfromClass "/Game/EVteam/comicPlayer/Tutos/tuto17AirJump.tuto17AirJump_C" (Transformation|GetActorTransform) "Undefined" 0 0))
        (Variables|/Game/EVteam/comicPlayer/Base/comicPlayer.comicPlayer_C|SetambSound _returnvalue (Variables|Default|GetambSoundRef))
        (Variables|Default|SetskillLevel 1)
        (Variables|Default|Setready4newSkill false))
      (:1
        (bind _returnvalue_2 (Game|SpawnActorfromClass "/Game/EVteam/comicPlayer/Tutos/tuto13qckRcvr.tuto13qckRcvr_C" (Transformation|GetActorTransform) "Undefined" 0 0))
        (Variables|/Game/EVteam/comicPlayer/Base/comicPlayer.comicPlayer_C|SetambSound _returnvalue_2 (Variables|Default|GetambSoundRef))
        (Variables|Default|Setready4newSkill false))
      (:2
        (bind _returnvalue_3 (Game|SpawnActorfromClass "/Game/EVteam/comicPlayer/Tutos/tuto14rise1.tuto14rise1_C" (Transformation|GetActorTransform) "Undefined" 0 0))
        (Variables|/Game/EVteam/comicPlayer/Base/comicPlayer.comicPlayer_C|SetambSound _returnvalue_3 (Variables|Default|GetambSoundRef))
        (Variables|Default|SetskillLevel 3)
        (Variables|Default|Setready4newSkill false))
      (:3
        (bind _returnvalue_4 (Game|SpawnActorfromClass "/Game/EVteam/comicPlayer/Tutos/tuto14rise2.tuto14rise2_C" (Transformation|GetActorTransform) "Undefined" 0 0))
        (Variables|/Game/EVteam/comicPlayer/Base/comicPlayer.comicPlayer_C|SetambSound _returnvalue_4 (Variables|Default|GetambSoundRef))
        (Variables|Default|SetskillLevel 4)
        (Variables|Default|Setready4newSkill false))
      (:4
        (bind _returnvalue_5 (Game|SpawnActorfromClass "/Game/EVteam/comicPlayer/Tutos/tuto14rise3.tuto14rise3_C" (Transformation|GetActorTransform) "Undefined" 0 0))
        (Variables|/Game/EVteam/comicPlayer/Base/comicPlayer.comicPlayer_C|SetambSound _returnvalue_5 (Variables|Default|GetambSoundRef))
        (Variables|Default|SetskillLevel 5)
        (Variables|Default|Setready4newSkill false)))
    (elif (and (Variables|Default|Getready2LearnGrabThrow) (not (Variables|Default|GetgrabThrowLearned)))
      (Variables|Default|SetgrabThrowLearned true)
      (Utilities|FlowControl|Delay 3.0)
      (bind _returnvalue_6 (Game|SpawnActorfromClass "/Game/EVteam/comicPlayer/Tutos/tuto16grabThrow.tuto16grabThrow_C" (Transformation|GetActorTransform) "Undefined" 0 0))
      (Variables|/Game/EVteam/comicPlayer/Base/comicPlayer.comicPlayer_C|SetambSound _returnvalue_6 (Variables|Default|GetambSoundRef))
      (elif (and (AI|Components|NavMovement|IsFalling (Variables|Character|GetCharacterMovement)) (== (Variables|Default|GetskillLevel) 0))
        (Utilities|FlowControl|Delay 0.5)
        (Variables|Default|Setready4newSkill true)))))

(event Input|KeyboardEvents|P
  (params (Key :type Key%20Structure))
  ;[1 1 1] Pause game
  (:Pressed
    (if (not (Variables|/Script/EpidemicVectors.VectorsGameStateBase|GetmotionComicLock (Variables|Default|GetgameState)))
      (bind _output_get (Variables|Default|Setpaused (not (Variables|Default|Getpaused))))
      (Development|PrintString (Utilities|String|Append "game paused is:" (Utilities|String|ToString(Boolean) _output_get)))
      (Game|SetGamePaused (Variables|Default|Getpaused)))))

(event Input|KeyboardEvents|SpaceBar
  (params (Key :type Key%20Structure))
  (:Pressed
    (Audio|PlaySoundatLocation 0 "0, 0, 0" "0, 0, 0" 1.0 1.0 0.0 0 0 0)))

(event Input|KeyboardEvents|M
  (params (Key :type Key%20Structure))
  ;[1 1 1] Reload Level
  (:Pressed
    (bind _returnvalue (Game|GetCurrentLevelName true))
    (Game|OpenLevel(byName) (Utilities|String|StringToName _returnvalue))))

(event Input|KeyboardEvents|I
  (params (Key :type Key%20Structure))
  (bind _ambsoundref (Variables|Default|GetambSoundRef))
  (bind _audiocomponent (Variables|/Script/Engine.AmbientSound|GetAudioComponent _ambsoundref))
  ;[1 1 1] Testing the comicPlayer example
  (:Pressed
    (bind _returnvalue (Game|SpawnActorfromClass "/Game/EVteam/comicPlayer/Base/comicPlayerTest.comicPlayerTest_C" (Transformation|GetActorTransform) "Undefined" 0 0))
    (Variables|/Game/EVteam/comicPlayer/Base/comicPlayer.comicPlayer_C|SetambSound _returnvalue _ambsoundref)
    (Variables|/Game/EVteam/comicPlayer/Base/comicPlayer.comicPlayer_C|SetbackMusic _returnvalue (Variables|/Script/Engine.AudioComponent|GetSound (Variables|/Script/Engine.AmbientSound|GetAudioComponent _ambsoundref)))
    (Audio|Components|Audio|FadeOut _audiocomponent 3.0 0.0 :!class /Script/Engine.AudioComponent)
    (Audio|Components|Audio|SetSound _audiocomponent (Variables|/Game/EVteam/comicPlayer/Base/comicPlayer.comicPlayer_C|GettutoBackMusic _returnvalue))))

(event Input|KeyboardEvents|N
  (params (Key :type Key%20Structure))
  ;[1 1 1] Reloads level from start, before all checkpoints
  (:Pressed
    (bind _returnvalue (SaveGame|CreateSaveGameObject "/Game/EVteam/blueprints/props/VectorsSave.VectorsSave_C"))
    (Variables|/Game/EVteam/blueprints/props/VectorsSave.VectorsSave_C|SetcheckPointID _returnvalue 0)
    (bind _returnvalue_2 (Game|GetCurrentLevelName true))
    (Variables|/Game/EVteam/blueprints/props/VectorsSave.VectorsSave_C|SetlevelName _returnvalue _returnvalue_2)
    (SaveGame|SaveGametoSlot _returnvalue "toLoad")
    (Game|OpenLevel(byName) (Utilities|String|StringToName _returnvalue_2))))

(event Input|KeyboardEvents|Z
  (params (Key :type Key%20Structure))
  (:Pressed
    (Class|GameplayStatics|SetGlobalPitchModulation 0.5 0.0))
  (:Released
    (Class|GameplayStatics|SetGlobalPitchModulation 1.0 0.0)))

(event Input|KeyboardEvents|Y
  (params (Key :type Key%20Structure))
  (:Pressed
    (Variables|Default|SetinteractionLevel (- (Variables|Default|GetinteractionLevel) 1))
    (Development|PrintString (Utilities|String|Append "interactionLevel: " (Utilities|String|ToString(Integer) (Variables|Default|GetinteractionLevel))))))

(event Input|KeyboardEvents|T
  (params (Key :type Key%20Structure))
  (:Pressed
    (Variables|Default|SetinteractionLevel (+ (Variables|Default|GetinteractionLevel) 1))
    (Development|PrintString (Utilities|String|Append "interactionLevel: " (Utilities|String|ToString(Integer) (Variables|Default|GetinteractionLevel))))))

(fn ConstructionScript)